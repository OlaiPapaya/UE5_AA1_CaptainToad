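; BP_Canonball is a cannonball projectile that flies straight and explodes on overlap or when its lifetime expires.
; Init stores the firing cannon and normalized direction, and Tick moves the ball without sweeping.
; Overlaps are ignored if that cannon is invalid or is the overlapped actor.
; Explode fires a radial impulse, spawns BP_SimpleExplosion, damages an overlapped third-person character, then destroys the ball.
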(event OnComponentBeginOverlap(StaticMesh)
  (params (OverlappedComponent :type Primitive%20Component%20Object%20Reference) (OtherActor :type Actor%20Object%20Reference) (OtherComp :type Primitive%20Component%20Object%20Reference) (OtherBodyIndex :type Integer) (bFromSweep :type Boolean) (SweepResult :type Hit%20Result%20Structure%20%28by%20ref%29))
  (if (Utilities|IsValid (Variables|Default|GetMyCanon))
    (bind _asbp_canon (Utilities|Casting|CastToBP_Canon OtherActor)
      (:then
        (if (not (== _asbp_canon (Variables|Default|GetMyCanon)))
          (CallFunction|Explode OtherActor :!label _label)))
      (:CastFailed
        (goto _label)))))

(event EventBeginPlay)

(event Collision|EventActorBeginOverlap
  (params (OtherActor :type Actor%20Object%20Reference)))

(event EventTick
  (params (DeltaSeconds :type Float%20%28single-precision%29))
  ;[0.15 0.15 0.15 0.5] Incrementing the lifetime counter and checking if it exceeded the maximum
  (bind _output_get (Variables|Default|SetCurrentLifetime (+ DeltaSeconds (Variables|Default|GetCurrentLifetime))))
  (if (< _output_get (Variables|Default|GetLifetime))
    ;[0.15 0.15 0.15 0.5] Moving the cannonball
    (Transformation|SetActorLocation (+ (Transformation|GetActorLocation) (* DeltaSeconds (Variables|Default|GetDirection) (Variables|Default|GetSpeed))) false false)
    (else
      (CallFunction|Explode))))

(fn ConstructionScript)

(fn Init
  (params (Canon :type BP%20Canon%20Object%20Reference) (Dir :type Vector))
  (Variables|Default|SetMyCanon Canon)
  (Variables|Default|SetDirection (Math|Vector|Normalize Dir)))

(fn Explode
  (params (OtherActor :type Actor%20Object%20Reference))
  (Utilities|FlowControl|Sequence
    (:then_0
      (Class|RadialForceComponent|FireImpulse (Variables|Default|GetRadialForce))
      (Game|SpawnActorfromClass "/Game/Blueprints/Others/BP_SimpleExplosion.BP_SimpleExplosion_C" (Transformation|GetActorTransform) "Undefined" "MultiplyWithRoot" 0 0))
    (:then_1
      (bind _asbp_third_person_character (Utilities|Casting|CastToBP_ThirdPersonCharacter OtherActor))
      (Game|Damage|ApplyDamage _asbp_third_person_character (Math|Conversions|ToFloat(Integer) (Variables|Default|GetDamageInflicted)) 0 0))
    (:then_2
      (Actor|DestroyActor))))