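; BP_Coins is a collectible coin that the third-person character picks up by touching it.
; On BeginPlay, the Float timeline drives the static mesh's relative height and yaw to animate it floating and rotating.
; When BP_ThirdPersonCharacter overlaps the Sphere, the coin calls GrabCoin on BP_CrystalsGameMode and destroys itself.
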(event OnComponentBeginOverlap(Sphere)
  (params (OverlappedComponent :type Primitive%20Component%20Object%20Reference) (OtherActor :type Actor%20Object%20Reference) (OtherComp :type Primitive%20Component%20Object%20Reference) (OtherBodyIndex :type Integer) (bFromSweep :type Boolean) (SweepResult :type Hit%20Result%20Structure%20%28by%20ref%29))
  (Utilities|Casting|CastToBP_ThirdPersonCharacter OtherActor)
  (bind _asbp_crystals_game_mode (Utilities|Casting|CastToBP_CrystalsGameMode (Game|GetGameMode)))
  (Default|GrabCoin _asbp_crystals_game_mode)
  (Actor|DestroyActor))

(event EventBeginPlay
  (bind (_direction _height _rotation) (Timeline|Float Play)
    (:Update
      (Transformation|SetRelativeLocation (Variables|Default|GetStaticMesh) (Math|Vector|MakeVector 0.0 0.0 _height) false false)
      (Transformation|SetRelativeRotation (Variables|Default|GetStaticMesh) (Math|Rotator|MakeRotator 0.0 0.0 _rotation) false false))))

(event Collision|EventActorBeginOverlap
  (params (OtherActor :type Actor%20Object%20Reference)))

(event EventTick
  (params (DeltaSeconds :type Float%20%28single-precision%29)))

(fn ConstructionScript)