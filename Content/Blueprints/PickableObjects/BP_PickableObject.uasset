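; BP_PickableObject is an actor that a carrier can pick up, hold overhead and throw.
; Pick stores the carrier and turns off mesh physics.
; While a carrier is set, Tick snaps the object to the carrier's location plus a height offset and copies its rotation, without attachment.
; Drop re-enables physics, applies a forward impulse from the carrier's facing, then clears the carrier.
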(event EventBeginPlay)

(event Collision|EventActorBeginOverlap
  (params (OtherActor :type Actor%20Object%20Reference)))

(event EventTick
  (params (DeltaSeconds :type Float%20%28single-precision%29))
  (bind _currentcarrier (Variables|Default|GetCurrentCarrier))
  (bind _returnvalue (Transformation|GetActorLocation _currentcarrier))
  (bind (_x _y _z) (Math|Vector|BreakVector _returnvalue))
  (if (Utilities|IsValid (Variables|Default|GetCurrentCarrier))
    (Transformation|SetActorLocation (Math|Vector|MakeVector _x _y (+ _z (Variables|Default|GetCarryHeight))) false false)
    (Transformation|SetActorRotation (Transformation|GetActorRotation (Variables|Default|GetCurrentCarrier)))))

(fn ConstructionScript)

(fn Pick
  (params (Carrier :type Actor%20Object%20Reference))
  (Variables|Default|SetCurrentCarrier Carrier)
  (Physics|SetSimulatePhysics (Variables|Default|GetStaticMesh) false))

(fn Drop
  (Utilities|FlowControl|Sequence
    (:then_0
      (Physics|SetSimulatePhysics (Variables|Default|GetStaticMesh) true)
      (if (Physics|IsSimulatingPhysics (Variables|Default|GetStaticMesh) "None")
        (Physics|AddImpulse (Variables|Default|GetStaticMesh) (* (Transformation|GetActorForwardVector (Variables|Default|GetCurrentCarrier)) (Variables|Default|GetDropForce)) "None" false)))
    (:then_1
      (Variables|Default|SetCurrentCarrier 0))))