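; BP_Button is a weight-activated pressure button that sends an on/off signal when its load crosses a threshold.
; Box overlaps from the player or physics-simulating components update CurrentWeight, using CharacterMovement mass for the player and physical mass otherwise.
; On exit, the total becomes the leaving mass minus CurrentWeight, the reverse of the commented intent.
; Both events share the threshold check, which toggles IsON, calls SendSignal and squashes or restores the mesh's Z scale.
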(event OnComponentBeginOverlap(Box)
  (params (OverlappedComponent :type Primitive%20Component%20Object%20Reference) (OtherActor :type Actor%20Object%20Reference) (OtherComp :type Primitive%20Component%20Object%20Reference) (OtherBodyIndex :type Integer) (bFromSweep :type Boolean) (SweepResult :type Hit%20Result%20Structure%20%28by%20ref%29))
  (bind _mesh (Variables|Default|GetMesh))
  (bind _mesh_2 (Variables|Default|GetMesh))
  (bind _relativescale3d (Variables|/Script/Engine.SceneComponent|GetRelativeScale3D _mesh))
  (bind _relativescale3d_2 (Variables|/Script/Engine.SceneComponent|GetRelativeScale3D _mesh_2))
  (bind (_x _y) (Math|Vector|BreakVector _relativescale3d))
  (bind (_x_2 _y_2) (Math|Vector|BreakVector _relativescale3d_2))
  ;[0.15 0.15 0.15 0.5] Checking if physics are enabled for this object or if it's a player
  (Utilities|Casting|CastToBP_ThirdPersonCharacter OtherActor
    (:then
      ;[0.15 0.15 0.15 0.5] Adding the object's weight to the current weight in hold
      (bind _mass (CallFunction|GetMass OtherComp :!label _label))
      (Variables|Default|SetCurrentWeight (+ _mass (Variables|Default|GetCurrentWeight)))
      (if (Variables|Default|GetIsON)
        ;[0.15 0.15 0.15 0.5] If the weight just got UNDER the threshold, we send the OFF signal
        (if (< (Variables|Default|GetCurrentWeight) (Variables|Default|GetThresholdWeight))
          (bind _output_get (Variables|Default|SetIsON false))
          (CallFunction|SendSignal _output_get)
          ;[0.15 0.15 0.15 0.5] Squash when pressed and stretch when not
          (Transformation|SetRelativeScale3D _mesh_2 (Math|Vector|MakeVector _x_2 _y_2 1.0)))
        (else
          ;[0.15 0.15 0.15 0.5] If the weight just got OVER the threshold, we send the ON signal
          (if (>= (Variables|Default|GetCurrentWeight) (Variables|Default|GetThresholdWeight))
            (bind _output_get_2 (Variables|Default|SetIsON true))
            (CallFunction|SendSignal _output_get_2)
            (Transformation|SetRelativeScale3D _mesh (Math|Vector|MakeVector _x _y 0.5))))))
    (:CastFailed
      (if (Physics|IsSimulatingPhysics OtherComp "None")
        (goto _label)))))

(event OnComponentEndOverlap(Box)
  (params (OverlappedComponent :type Primitive%20Component%20Object%20Reference) (OtherActor :type Actor%20Object%20Reference) (OtherComp :type Primitive%20Component%20Object%20Reference) (OtherBodyIndex :type Integer))
  (bind _mesh (Variables|Default|GetMesh))
  (bind _mesh_2 (Variables|Default|GetMesh))
  (bind _relativescale3d (Variables|/Script/Engine.SceneComponent|GetRelativeScale3D _mesh))
  (bind _relativescale3d_2 (Variables|/Script/Engine.SceneComponent|GetRelativeScale3D _mesh_2))
  (bind (_x _y) (Math|Vector|BreakVector _relativescale3d))
  (bind (_x_2 _y_2) (Math|Vector|BreakVector _relativescale3d_2))
  ;[0.15 0.15 0.15 0.5] Checking if physics are enabled for this object or if it's a player
  (Utilities|Casting|CastToBP_ThirdPersonCharacter OtherActor
    (:then
      ;[0.15 0.15 0.15 0.5] Substracting the object's weight from the current weight in hold
      (bind _mass (CallFunction|GetMass OtherComp :!label _label))
      (Variables|Default|SetCurrentWeight (- _mass (Variables|Default|GetCurrentWeight)))
      (if (Variables|Default|GetIsON)
        ;[0.15 0.15 0.15 0.5] If the weight just got UNDER the threshold, we send the OFF signal
        (if (< (Variables|Default|GetCurrentWeight) (Variables|Default|GetThresholdWeight))
          (bind _output_get (Variables|Default|SetIsON false))
          (CallFunction|SendSignal _output_get)
          ;[0.15 0.15 0.15 0.5] Squash when pressed and stretch when not
          (Transformation|SetRelativeScale3D _mesh_2 (Math|Vector|MakeVector _x_2 _y_2 1.0)))
        (else
          ;[0.15 0.15 0.15 0.5] If the weight just got OVER the threshold, we send the ON signal
          (if (>= (Variables|Default|GetCurrentWeight) (Variables|Default|GetThresholdWeight))
            (bind _output_get_2 (Variables|Default|SetIsON true))
            (CallFunction|SendSignal _output_get_2)
            (Transformation|SetRelativeScale3D _mesh (Math|Vector|MakeVector _x _y 0.5))))))
    (:CastFailed
      (if (Physics|IsSimulatingPhysics OtherComp "None")
        (goto _label)))))

(event EventBeginPlay)

(event Collision|EventActorBeginOverlap
  (params (OtherActor :type Actor%20Object%20Reference)))

(event EventTick
  (params (DeltaSeconds :type Float%20%28single-precision%29)))

(fn ConstructionScript)

(fn GetMass
  (params (OtherObj :type Primitive%20Component%20Object%20Reference))
  ;[0.15 0.15 0.15 0.5] The player itself doesn't have physics enabled, so we read its Mass variable from the Character Movement settings
  (bind _asbp_third_person_character (Utilities|Casting|CastToBP_ThirdPersonCharacter (Components|GetOwner OtherObj))
    (:then
      (return (Variables|/Script/Engine.CharacterMovementComponent|GetMass (Variables|/Script/Engine.Character|GetCharacterMovement _asbp_third_person_character))))
    (:CastFailed
      ;[0.15 0.15 0.15 0.5] If it's not the player, we get the object's physical mass
      (return (Physics|GetMass OtherObj)))))