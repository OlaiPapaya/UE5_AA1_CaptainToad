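; Actor component that tracks health for its owner and reports changes and death through event dispatchers.
; On BeginPlay it fills CurrentHealth to MaxHealth and binds to the owner's OnTakeAnyDamage, subtracting truncated damage as integers.
; Add and remove functions clamp health to the valid range, broadcast HealthChanged, then fire Died at zero, with no guard against repeat broadcasts.
; Kill zeroes health and fires both dispatchers directly.
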(event Custom|OnTakeDamage
  (params (DamagedActor :type Actor%20Object%20Reference) (Damage :type Float%20%28single-precision%29) (DamageType :type Damage%20Type%20Object%20Reference) (InstigatedBy :type Controller%20Object%20Reference) (DamageCauser :type Actor%20Object%20Reference))
  (CallFunction|RemoveHealth (Math|Float|Truncate Damage)))

(event EventBeginPlay
  (EventDispatchers|BindEventtoOnTakeAnyDamage (Components|GetOwner) (delegate Custom|OnTakeDamage))
  (Variables|Default|SetCurrentHealth (Variables|Default|GetMaxHealth)))

(event EventTick
  (params (DeltaSeconds :type Float%20%28single-precision%29)))

(fn AddHealth
  (params (Health :type Integer))
  (bind _output_get (Variables|Default|SetCurrentHealth (Math|Integer|Clamp(Integer) (+ (Variables|Default|GetCurrentHealth) Health) 0 (Variables|Default|GetMaxHealth))))
  (Default|CallHealthChanged _output_get)
  (CallFunction|CheckKill))

(fn RemoveHealth
  (params (Health :type Integer))
  (bind _output_get (Variables|Default|SetCurrentHealth (Math|Integer|Clamp(Integer) (- (Variables|Default|GetCurrentHealth) Health) 0 (Variables|Default|GetMaxHealth))))
  (Default|CallHealthChanged _output_get)
  (CallFunction|CheckKill))

(fn Kill
  (bind _output_get (Variables|Default|SetCurrentHealth 0))
  (Default|CallHealthChanged _output_get)
  (Default|CallDied))

(fn CheckKill
  (if (<= (Variables|Default|GetCurrentHealth) 0)
    (Default|CallDied)))