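; BP_ElevatorLever is an elevator that moves vertically when switched on or off, with a lever attached as a child actor.
; On BeginPlay it adds itself to that BP_Lever's EnabledActors list.
; SwitchON and SwitchOFF play separate timelines that raise and lower the whole actor by VerticalDistance.
; Each update adds only the change since the previous frame to the current location rather than setting an absolute position.
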(event EventBeginPlay
  (bind _asbp_lever (Utilities|Casting|CastToBP_Lever (Variables|/Script/Engine.ChildActorComponent|GetChildActor (Variables|Default|GetLever))))
  (Utilities|Array|Add (Variables|/Game/Blueprints/InteractableObjects/BP_InteractableObject.BP_InteractableObject_C|GetEnabledActors _asbp_lever) self))

(event Collision|EventActorBeginOverlap
  (params (OtherActor :type Actor%20Object%20Reference))
  (|CallParentFunction OtherActor) ; This node is disabled and will not be called.\nDrag off pins to build functionality.
)

(event EventTick
  (params (DeltaSeconds :type Float%20%28single-precision%29))
  (|CallParentFunction DeltaSeconds) ; This node is disabled and will not be called.\nDrag off pins to build functionality.
)

(event EventSwitchOFF
  (bind _position (Timeline|Timeline PlayFromStart)
    (:Update
      ;[0.15 0.15 0.15 0.5] Instead of hard-setting the rotation, we just add the difference since the last frame. This way two rotations can coexist.
      (Transformation|SetActorLocation (+ (Math|Vector|MakeVector 0.0 0.0 (- (Variables|Default|GetDownwardsMovement) (* _position (Variables|Default|GetVerticalDistance)))) (Transformation|GetActorLocation)) false false)
      (Variables|Default|SetDownwardsMovement (* _position (Variables|Default|GetVerticalDistance))))
    (:Finished
      (Variables|Default|SetDownwardsMovement 0.0))))

(event EventSwitchON
  (bind _position (Timeline|Position PlayFromStart)
    (:Update
      ;[0.15 0.15 0.15 0.5] Instead of hard-setting the rotation, we just add the difference since the last frame. This way two rotations can coexist.
      (Transformation|SetActorLocation (+ (Math|Vector|MakeVector 0.0 0.0 (- (* _position (Variables|Default|GetVerticalDistance)) (Variables|Default|GetUpwardsMovement))) (Transformation|GetActorLocation)) false false)
      (Variables|Default|SetUpwardsMovement (* _position (Variables|Default|GetVerticalDistance))))
    (:Finished
      (Variables|Default|SetUpwardsMovement 0.0))))

(fn ConstructionScript
  (|CallParentFunction))