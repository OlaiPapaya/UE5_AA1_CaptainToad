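; BP_RotatoryPlatformLong is a non-interactable platform that rotates in yaw in response to an on/off signal.
; PerformAction plays the Rotate timeline when on; when off it plays RotateBackwards if UndoRotation is set, otherwise it clears RespondingToSignal.
; Both timelines add only the local rotation delta since the last update, so two rotations can coexist.
; Each resets its tracked angle and clears RespondingToSignal on finishing.
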(event EventBeginPlay
  (|CallParentFunction) ; This node is disabled and will not be called.\nDrag off pins to build functionality.
)

(event Collision|EventActorBeginOverlap
  (params (OtherActor :type Actor%20Object%20Reference))
  (|CallParentFunction OtherActor) ; This node is disabled and will not be called.\nDrag off pins to build functionality.
)

(event EventTick
  (params (DeltaSeconds :type Float%20%28single-precision%29))
  (|CallParentFunction DeltaSeconds) ; This node is disabled and will not be called.\nDrag off pins to build functionality.
)

(fn ConstructionScript
  (|CallParentFunction))

(fn PerformAction
  (params (IsON :type Boolean))
  (if IsON
    (Components|Timeline|PlayfromStart (Variables|Default|GetRotate))
    (elif (Variables|Default|GetUndoRotation)
      (Components|Timeline|PlayfromStart (Variables|Default|GetRotateBackwards))
      (else
        (Variables|Default|SetRespondingToSignal false)))))