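; BP_Canon is a cannon that periodically fires BP_Canonball projectiles.
; On BeginPlay a looping timer calls ShootBall at the ShootingCadence interval.
; ShootBall spawns a ball at the cannon's transform and initializes it with the cannon reference and its forward vector as direction.
; SwitchON pauses the timer and SwitchOFF resumes it, so switching on halts firing.
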(event EventBeginPlay
  (bind _returnvalue (Utilities|Time|SetTimerbyFunctionName 0 "ShootBall" (Variables|Default|GetShootingCadence) true))
  (Variables|Default|SetTimerHandle _returnvalue))

(event EventSwitchOFF
  (Utilities|Time|UnpauseTimerbyHandle (Variables|Default|GetTimerHandle)))

(event EventSwitchON
  (Utilities|Time|PauseTimerbyHandle (Variables|Default|GetTimerHandle)))

(fn ConstructionScript
  (|CallParentFunction))

(fn ShootBall
  (bind _returnvalue (Game|SpawnActorfromClass "/Game/Blueprints/Others/BP_Canonball.BP_Canonball_C" (Transformation|GetActorTransform) "Undefined" "MultiplyWithRoot" 0 0))
  (Default|Init _returnvalue self (Transformation|GetActorForwardVector)))