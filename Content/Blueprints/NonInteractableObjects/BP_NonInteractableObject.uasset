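; Base Blueprint for non-interactable objects that react to on/off signals.
; SwitchON and SwitchOFF append booleans to an ArrivedSignals queue, which Tick polls while no signal is being handled.
; RespondToSignal sets a busy flag, passes the oldest signal to PerformAction and removes it.
; PerformAction is an empty stub and nothing here clears the busy flag; Tick also prints a debug "Hello".
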(event EventBeginPlay)

(event Collision|EventActorBeginOverlap
  (params (OtherActor :type Actor%20Object%20Reference)))

(event EventTick
  (params (DeltaSeconds :type Float%20%28single-precision%29))
  (if (and (not (Variables|Default|GetRespondingToSignal)) (Utilities|Array|IsNotEmpty (Variables|Default|GetArrivedSignals)))
    (CallFunction|RespondtoSignal)
    (Development|PrintString "Hello")))

(event EventSwitchOFF
  (Utilities|Array|Add (Variables|Default|GetArrivedSignals) false))

(event EventSwitchON
  (Utilities|Array|Add (Variables|Default|GetArrivedSignals) true))

(fn ConstructionScript)

(fn RespondtoSignal
  (Variables|Default|SetRespondingToSignal true)
  (CallFunction|PerformAction (Utilities|Array|Get(acopy) (Variables|Default|GetArrivedSignals)))
  (Utilities|Array|RemoveIndex (Variables|Default|GetArrivedSignals)))

(fn PerformAction
  (params (IsON :type Boolean)))