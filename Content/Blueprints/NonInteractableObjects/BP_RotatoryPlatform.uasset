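; A switchable platform actor that yaws in place when switched on and can turn back when switched off.
; SwitchON plays a timeline from the start to turn it; SwitchOFF, only if UndoRotation is set, plays a second timeline applied in the opposite direction.
; Each update adds only the change since that timeline's last value as local rotation, so the two rotations can coexist instead of overwriting each other.
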(event EventBeginPlay
  (|CallParentFunction) ; This node is disabled and will not be called.\nDrag off pins to build functionality.
)

(event Collision|EventActorBeginOverlap
  (params (OtherActor :type Actor%20Object%20Reference))
  (|CallParentFunction OtherActor) ; This node is disabled and will not be called.\nDrag off pins to build functionality.
)

(event EventTick
  (params (DeltaSeconds :type Float%20%28single-precision%29))
  (|CallParentFunction DeltaSeconds) ; This node is disabled and will not be called.\nDrag off pins to build functionality.
)

(event EventSwitchOFF
  (if (Variables|Default|GetUndoRotation)
    (bind _rotation (Timeline|Rotation PlayFromStart)
      (:Update
        ;[0.15 0.15 0.15 0.5] Instead of hard-setting the rotation, we just add the difference since the last frame. This way two rotations can coexist.
        (Transformation|AddActorLocalRotation (Math|Rotator|MakeRotator 0.0 0.0 (- (Variables|Default|GetCounterclockwardsRotation) _rotation)) false false)
        (Variables|Default|SetCounterclockwardsRotation _rotation)))))

(event EventSwitchON
  (bind _rotation (Timeline|Timeline PlayFromStart)
    (:Update
      ;[0.15 0.15 0.15 0.5] Instead of hard-setting the rotation, we just add the difference since the last frame. This way two rotations can coexist.
      (Transformation|AddActorLocalRotation (Math|Rotator|MakeRotator 0.0 0.0 (- _rotation (Variables|Default|GetClockwardsRotation))) false false)
      (Variables|Default|SetClockwardsRotation _rotation))))

(fn ConstructionScript
  (|CallParentFunction))