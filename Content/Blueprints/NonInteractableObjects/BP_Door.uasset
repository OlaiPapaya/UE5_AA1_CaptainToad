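; Door actor that swings open on SwitchON and swings back on SwitchOFF.
; Each event plays its own timeline from the start, turning the DoorClosed component around local yaw, with the close delta negated.
; Rotation is applied as the change since the last update, tracked in OpenRotation and CloseRotation, which reset to zero only when their timeline finishes.
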(event EventBeginPlay
  (|CallParentFunction) ; This node is disabled and will not be called.\nDrag off pins to build functionality.
)

(event Collision|EventActorBeginOverlap
  (params (OtherActor :type Actor%20Object%20Reference))
  (|CallParentFunction OtherActor) ; This node is disabled and will not be called.\nDrag off pins to build functionality.
)

(event EventTick
  (params (DeltaSeconds :type Float%20%28single-precision%29))
  (|CallParentFunction DeltaSeconds) ; This node is disabled and will not be called.\nDrag off pins to build functionality.
)

(event EventSwitchOFF
  (bind _rotation (Timeline|Timeline PlayFromStart)
    (:Update
      (Transformation|AddLocalRotation (Variables|Default|GetDoorClosed) (Math|Rotator|MakeRotator 0.0 0.0 (- (Variables|Default|GetCloseRotation) _rotation)) false false)
      (Variables|Default|SetCloseRotation _rotation))
    (:Finished
      (Variables|Default|SetCloseRotation 0.0))))

(event EventSwitchON
  (bind _rotation (Timeline|OpenDoor PlayFromStart)
    (:Update
      (Transformation|AddLocalRotation (Variables|Default|GetDoorClosed) (Math|Rotator|MakeRotator 0.0 0.0 (- _rotation (Variables|Default|GetOpenRotation))) false false)
      (Variables|Default|SetOpenRotation _rotation))
    (:Finished
      (Variables|Default|SetOpenRotation 0.0))))

(fn ConstructionScript
  (|CallParentFunction))