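; Game mode for a crystal-collecting game that handles pickup scoring and the win and lose outcomes.
; On BeginPlay it adds crystal and coin counter widgets and binds to the Died event of the player character's AC_Health component.
; GrabCrystal and GrabCoin update BP_CrystalsGameState, with GrabCrystal calling Win at the crystal target.
; Win and Lost each check a shared GameEnded flag, then pause the game and show their result widget.
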(event EventBeginPlay
  (Utilities|FlowControl|Sequence
    (:then_0
      (bind _returnvalue (UserInterface|CreateWidget "/Game/UI/WBP_CrystalCounter.WBP_CrystalCounter_C"))
      (UserInterface|Viewport|AddtoViewport _returnvalue 0))
    (:then_1
      (bind _returnvalue_2 (UserInterface|CreateWidget "/Game/UI/WBP_CoinsCounter.WBP_CoinsCounter_C"))
      (UserInterface|Viewport|AddtoViewport _returnvalue_2 0))
    (:then_2
      (bind _asbp_third_person_character (Utilities|Casting|CastToBP_ThirdPersonCharacter (Game|Player|GetPlayerPawn 0)))
      (EventDispatchers|BindEventtoDied (Actor|GetComponentbyClass _asbp_third_person_character "/Game/Blueprints/ActorComponents/AC_Health.AC_Health_C") (EventDispatchers|CreateEvent :!event Lost)))))

(event EventTick
  (params (DeltaSeconds :type Float%20%28single-precision%29)))

(fn ConstructionScript)

(fn GrabCrystal
  (bind _asbp_crystals_game_state (Utilities|Casting|CastToBP_CrystalsGameState (Game|GetGameState)))
  (Default|AddCrystal _asbp_crystals_game_state)
  (if (>= (Variables|/Game/GameFramework/BP_CrystalsGameState.BP_CrystalsGameState_C|GetCrystalsCollected _asbp_crystals_game_state) (Variables|/Game/GameFramework/BP_CrystalsGameState.BP_CrystalsGameState_C|GetCrystalsToWin _asbp_crystals_game_state))
    (CallFunction|Win)))

(fn Win
  (bind _asbp_crystals_game_state (Utilities|Casting|CastToBP_CrystalsGameState (Game|GetGameState)))
  (if (not (Variables|/Game/GameFramework/BP_CrystalsGameState.BP_CrystalsGameState_C|GetGameEnded _asbp_crystals_game_state))
    (Variables|/Game/GameFramework/BP_CrystalsGameState.BP_CrystalsGameState_C|SetGameEnded _asbp_crystals_game_state true)
    (Game|SetGamePaused true)
    (bind _returnvalue (UserInterface|CreateWidget "/Game/UI/WBP_Win.WBP_Win_C"))
    (UserInterface|Viewport|AddtoViewport _returnvalue 0)))

(fn GrabCoin
  (bind _asbp_crystals_game_state (Utilities|Casting|CastToBP_CrystalsGameState (Game|GetGameState)))
  (Default|AddCoin _asbp_crystals_game_state))

(fn Lost
  (bind _asbp_crystals_game_state (Utilities|Casting|CastToBP_CrystalsGameState (Game|GetGameState)))
  (if (not (Variables|/Game/GameFramework/BP_CrystalsGameState.BP_CrystalsGameState_C|GetGameEnded _asbp_crystals_game_state))
    (Variables|/Game/GameFramework/BP_CrystalsGameState.BP_CrystalsGameState_C|SetGameEnded _asbp_crystals_game_state true)
    (Game|SetGamePaused true)
    (bind _returnvalue (UserInterface|CreateWidget "/Game/UI/WBP_Lose.WBP_Lose_C"))
    (UserInterface|Viewport|AddtoViewport _returnvalue 0)))